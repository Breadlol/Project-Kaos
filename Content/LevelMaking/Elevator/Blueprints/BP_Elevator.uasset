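; BP_Elevator is a trigger-driven elevator that also starts the boss battle music.
; When BP_FirstPersonCharacter enters the Box, the Elevator timeline plays after a short delay, setting the Cube's relative location.
; Leaving the Box reverses the timeline after the same delay.
; The first overlap by any actor plays the music once, guarded by MusicStarted, because that sequence branch skips the character cast.
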(event OnComponentBeginOverlap(Box)
  (params (OverlappedComponent :type Primitive%20Component%20Object%20Reference) (OtherActor :type Actor%20Object%20Reference) (OtherComp :type Primitive%20Component%20Object%20Reference) (OtherBodyIndex :type Integer) (bFromSweep :type Boolean) (SweepResult :type Hit%20Result%20Structure%20%28by%20ref%29))
  (Utilities|FlowControl|Sequence
    (:then_0
      (Utilities|Casting|CastToBP_FirstPersonCharacter OtherActor)
      (Utilities|FlowControl|Delay 0.2)
      (bind _elevator (Timeline|Elevator Play)
        (:Update
          (Transformation|SetRelativeLocation (Variables|Default|GetCube) _elevator false false))))
    (:then_1
      (if (not (Variables|Default|GetMusicStarted))
        (Audio|PlaySound2D "/Game/Boss_Battle_Final_Track_Cue.Boss_Battle_Final_Track_Cue" 1.0 1.0 0.0 0 0)
        (Variables|Default|SetMusicStarted true)))))

(event OnComponentEndOverlap(Box)
  (params (OverlappedComponent :type Primitive%20Component%20Object%20Reference) (OtherActor :type Actor%20Object%20Reference) (OtherComp :type Primitive%20Component%20Object%20Reference) (OtherBodyIndex :type Integer))
  (Utilities|Casting|CastToBP_FirstPersonCharacter OtherActor)
  (Utilities|FlowControl|Delay 0.2)
  (bind _elevator (Timeline|Elevator Reverse)
    (:Update
      (Transformation|SetRelativeLocation (Variables|Default|GetCube) _elevator false false))))

(fn ConstructionScript)