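; Trigger actor that plays a level sequence cutscene with accompanying dialogue when its box is overlapped.
; BeginPlay prepares the sequence player and a NormalDialogue widget linked to an NPC_Dialogue instance; overlap disables player input, plays the sequence and activates that widget.
; Its own chat events show or remove NPC_Dialogue, toggling movement, cursor and input mode.
; Code setting the chat's back-reference to this trigger is unconnected.
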(event OnComponentBeginOverlap(Box)
  (params (OverlappedComponent :type Primitive%20Component%20Object%20Reference) (OtherActor :type Actor%20Object%20Reference) (OtherComp :type Primitive%20Component%20Object%20Reference) (OtherBodyIndex :type Integer) (bFromSweep :type Boolean) (SweepResult :type Hit%20Result%20Structure%20%28by%20ref%29))
  (Input|DisableInput (Game|GetPlayerCharacter 0) (Game|GetPlayerController 0))
  (Sequencer|Player|Play (Variables|Default|GetCutscene) :!class /Script/MovieScene.MovieSceneSequencePlayer)
  (Default|ActivateDialogue (stale EventBeginPlay _returnvalue_3)))

(event Custom|EndChat
  (bind _returnvalue (Game|GetPlayerController 0))
  (Widget|RemovefromParent (Variables|Default|GetNPCChat))
  (Pawn|Components|CharacterMovement|SetMovementMode (Variables|/Script/Engine.Character|GetCharacterMovement (Game|GetPlayerCharacter 0)) "MOVE_Walking" 0)
  (Variables|/Script/Engine.PlayerController|SetbShowMouseCursor _returnvalue false)
  (Input|EnableInput (Game|GetPlayerCharacter 0) _returnvalue)
  (Input|SetInputModeGameOnly (Game|GetPlayerController 0)))

(event Custom|BeginChat
  (bind _npcchat (Variables|Default|GetNPCChat))
  (Default|Begin _npcchat false (Variables|Default|GetDialogue) false)
  (UserInterface|Viewport|AddtoViewport _npcchat 0))

(event Custom|Activate%20Dialogue
  (CallFunction|PlayerAdjustments)
  (CallFunction|BeginChat))

(event Custom|PlayerAdjustments
  (bind _returnvalue (Game|GetPlayerController 0))
  (Variables|/Script/Engine.PlayerController|SetbShowMouseCursor _returnvalue true)
  (Pawn|Components|CharacterMovement|DisableMovement (Variables|/Script/Engine.Character|GetCharacterMovement (Game|GetPlayerCharacter 0)))
  (Input|SetInputModeUIOnly _returnvalue 0 "DoNotLock"))

(event EventBeginPlay
  (bind _returnvalue (Sequencer|Player|CreateLevelSequencePlayer (Variables|Default|GetLevel%20Sequence)))
  (Variables|Default|SetCutscene _returnvalue)
  (bind _returnvalue_2 (Game|ConstructObjectfromClass "/Game/NPC-Interaction-UI/Blueprints/NPC_Dialogue.NPC_Dialogue_C"))
  (Variables|Default|SetNPCChat _returnvalue_2)
  (bind _returnvalue_3 (UserInterface|CreateWidget "/Game/CutsceneDialogue/Blueprints/NormalDialogue.NormalDialogue_C"))
  (Variables|/Game/CutsceneDialogue/Blueprints/NormalDialogue.NormalDialogue_C|SetDialogue _returnvalue_3 (Variables|Default|GetDialogue))
  (Variables|/Game/CutsceneDialogue/Blueprints/NormalDialogue.NormalDialogue_C|Setautoplay? _returnvalue_3 false)
  (Variables|/Game/CutsceneDialogue/Blueprints/NormalDialogue.NormalDialogue_C|SetNPCChat _returnvalue_3 (Variables|Default|GetNPCChat)))

(fn ConstructionScript)