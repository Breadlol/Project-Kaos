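; Behavior Tree task that updates a Patrol_Enemey's patrol index, by its name when a path point is reached.
; It advances CurrentPathIndex by PathDirection while the resulting PatrolPatha index is valid.
; At a path end, PatrolPathBehavior either leaves the index as is, flips the direction without moving the index, or resets the index to zero to loop.
; Each of these branches finishes successfully.
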(event EventReceiveExecuteAI
  (params (OwnerController :type AI%20Controller%20Object%20Reference) (ControlledPawn :type Pawn%20Object%20Reference))
  (bind _aspatrol_enemey (Utilities|Casting|CastToPatrol_Enemey ControlledPawn))
  (bind _output_get (Variables|Default|SetAs%20Patrol%20Enemey _aspatrol_enemey))
  (if (Utilities|Array|IsValidIndex (Variables|/Game/Blueprints/PatrolAIAssets/Patrol_Enemey.Patrol_Enemey_C|GetPatrolPatha _output_get) (+ (Variables|/Game/Blueprints/PatrolAIAssets/Patrol_Enemey.Patrol_Enemey_C|GetCurrentPathIndex _output_get) (Variables|/Game/Blueprints/PatrolAIAssets/Patrol_Enemey.Patrol_Enemey_C|GetPathDirection _output_get)))
    (Variables|/Game/Blueprints/PatrolAIAssets/Patrol_Enemey.Patrol_Enemey_C|SetCurrentPathIndex (Variables|Default|GetAs%20Patrol%20Enemey) (+ (Variables|/Game/Blueprints/PatrolAIAssets/Patrol_Enemey.Patrol_Enemey_C|GetCurrentPathIndex (Variables|Default|GetAs%20Patrol%20Enemey)) (Variables|/Game/Blueprints/PatrolAIAssets/Patrol_Enemey.Patrol_Enemey_C|GetPathDirection (Variables|Default|GetAs%20Patrol%20Enemey))))
    (AI|BehaviorTree|FinishExecute true)
    (else
      (switch Utilities|FlowControl|Switch|SwitchonPatrolPathEnding (Variables|/Game/Blueprints/PatrolAIAssets/Patrol_Enemey.Patrol_Enemey_C|GetPatrolPathBehavior (Variables|Default|GetAs%20Patrol%20Enemey))
        (:NewEnumerator0
          (AI|BehaviorTree|FinishExecute true))
        (:NewEnumerator1
          (Variables|/Game/Blueprints/PatrolAIAssets/Patrol_Enemey.Patrol_Enemey_C|SetPathDirection (Variables|Default|GetAs%20Patrol%20Enemey) (* (Variables|/Game/Blueprints/PatrolAIAssets/Patrol_Enemey.Patrol_Enemey_C|GetPathDirection (Variables|Default|GetAs%20Patrol%20Enemey)) -1))
          (AI|BehaviorTree|FinishExecute true))
        (:NewEnumerator2
          (Variables|/Game/Blueprints/PatrolAIAssets/Patrol_Enemey.Patrol_Enemey_C|SetCurrentPathIndex (Variables|Default|GetAs%20Patrol%20Enemey) 0)
          (AI|BehaviorTree|FinishExecute true))))))