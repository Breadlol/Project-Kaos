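; Behavior tree task that sets up the next patrol stop for a Patrol_Enemey from the path point at its current index.
; It writes a random navigable location near that point to the target key and a wait time randomized by the point's deviation to the wait key.
; It also applies walk speed and clears the caution state, then finishes successfully without advancing the path index.
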(event EventReceiveExecuteAI
  (params (OwnerController :type AI%20Controller%20Object%20Reference) (ControlledPawn :type Pawn%20Object%20Reference))
  (bind _aspatrol_enemey (Utilities|Casting|CastToPatrol_Enemey ControlledPawn))
  (bind _output_get (Variables|Default|SetAs%20Patrol%20Enemey _aspatrol_enemey))
  (AI|BehaviorTree|SetBlackboardValueasVector (Variables|Default|GetBB_target) (.RandomLocation (Class|NavigationSystemV1|GetRandomPointinNavigableRadius (Transformation|GetActorLocation (Utilities|Array|Get(acopy) (Variables|/Game/Blueprints/PatrolAIAssets/Patrol_Enemey.Patrol_Enemey_C|GetPatrolPatha _output_get) (Variables|/Game/Blueprints/PatrolAIAssets/Patrol_Enemey.Patrol_Enemey_C|GetCurrentPathIndex _output_get))) 5e+01 0 0)))
  (Class|BTFunctionLibrary|SetBlackboardValueasFloat (Variables|Default|GetBB_WaitTime) (Math|Random|RandomFloatinRange (- (Variables|/Game/Blueprints/PatrolAIAssets/StealthPathPnt.StealthPathPnt_C|GetWaitTime (Utilities|Array|Get(acopy) (Variables|/Game/Blueprints/PatrolAIAssets/Patrol_Enemey.Patrol_Enemey_C|GetPatrolPatha (Variables|Default|GetAs%20Patrol%20Enemey)) (Variables|/Game/Blueprints/PatrolAIAssets/Patrol_Enemey.Patrol_Enemey_C|GetCurrentPathIndex (Variables|Default|GetAs%20Patrol%20Enemey)))) (Variables|/Game/Blueprints/PatrolAIAssets/StealthPathPnt.StealthPathPnt_C|GetWaitDeviation (Utilities|Array|Get(acopy) (Variables|/Game/Blueprints/PatrolAIAssets/Patrol_Enemey.Patrol_Enemey_C|GetPatrolPatha (Variables|Default|GetAs%20Patrol%20Enemey)) (Variables|/Game/Blueprints/PatrolAIAssets/Patrol_Enemey.Patrol_Enemey_C|GetCurrentPathIndex (Variables|Default|GetAs%20Patrol%20Enemey))))) (+ (Variables|/Game/Blueprints/PatrolAIAssets/StealthPathPnt.StealthPathPnt_C|GetWaitTime (Utilities|Array|Get(acopy) (Variables|/Game/Blueprints/PatrolAIAssets/Patrol_Enemey.Patrol_Enemey_C|GetPatrolPatha (Variables|Default|GetAs%20Patrol%20Enemey)) (Variables|/Game/Blueprints/PatrolAIAssets/Patrol_Enemey.Patrol_Enemey_C|GetCurrentPathIndex (Variables|Default|GetAs%20Patrol%20Enemey)))) (Variables|/Game/Blueprints/PatrolAIAssets/StealthPathPnt.StealthPathPnt_C|GetWaitDeviation (Utilities|Array|Get(acopy) (Variables|/Game/Blueprints/PatrolAIAssets/Patrol_Enemey.Patrol_Enemey_C|GetPatrolPatha (Variables|Default|GetAs%20Patrol%20Enemey)) (Variables|/Game/Blueprints/PatrolAIAssets/Patrol_Enemey.Patrol_Enemey_C|GetCurrentPathIndex (Variables|Default|GetAs%20Patrol%20Enemey)))))))
  (Variables|/Script/Engine.CharacterMovementComponent|SetMaxWalkSpeed (Variables|/Script/Engine.Character|GetCharacterMovement (Variables|Default|GetAs%20Patrol%20Enemey)) (Variables|Default|GetWalkSpeed))
  (Class|BTFunctionLibrary|SetBlackboardValueasBool (Variables|Default|GetBB_CautionState) false)
  (AI|BehaviorTree|FinishExecute true))