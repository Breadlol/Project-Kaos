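; BP_FriendlyKaos_AI is a friendly NPC Blueprint that moves along a spline passed into its MoveObject event.
; When UseSpline is set, a timeline plays at a rate derived from TimeToCompleteSplineInSeconds.
; Each update maps the timeline track to a distance along the spline and sets the actor's world location and rotation to match.
; The construction script is empty.
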(event Custom|Move%20Object
  (params (Spline%20REF :type BP%20Spline%20Path%20Object%20Reference))
  (bind _spline (Variables|/Game/AI_NPC/Friendly_AI/BP_Spline_Path.BP_Spline_Path_C|GetSpline Spline%20REF))
  ;[0.9332 0.487 1] Move Along the Spline (It connects to the center of the mesh)
  (if (Variables|SplinePath|GetUse%20Spline?)
    (Components|Timeline|SetPlayRate (Variables|Default|GetMove%20Object%20T) (/ 1.0 (Variables|SplinePath|GetTime%20to%20Complete%20Spline%20%28in%20Seconds%29)))
    (bind _move_track (Timeline|Move%20Object%20T Play)
      (:Update
        (Transformation|SetActorTransform (Math|Transform|MakeTransform (Spline|GetLocationatDistanceAlongSpline _spline (Math|Float|Lerp 0.0 (Spline|GetSplineLength (Variables|/Game/AI_NPC/Friendly_AI/BP_Spline_Path.BP_Spline_Path_C|GetSpline Spline%20REF)) _move_track) "World") (Spline|GetRotationatDistanceAlongSpline _spline (Math|Float|Lerp 0.0 (Spline|GetSplineLength (Variables|/Game/AI_NPC/Friendly_AI/BP_Spline_Path.BP_Spline_Path_C|GetSpline Spline%20REF)) _move_track) "World") "1.000000,1.000000,1.000000"))))))

(fn ConstructionScript)